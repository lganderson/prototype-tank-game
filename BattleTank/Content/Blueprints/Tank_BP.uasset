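; Tank pawn Blueprint that assembles the tank from separate mesh parts and lets the player orbit the aiming camera.
; The construction script attaches the turret and both tracks to body sockets, and the barrel to a socket on the turret.
; AimAzimuth axis input yaws an azimuth gimbal, while AimElevation pitches the spring arm, keeping the two rotation axes separate.
; The turret and barrel are not rotated here, and the event graph holds only disabled stubs.
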(event `InputAxis|AimAzimuth`
  (params (AxisValue :type "Float (single-precision)"))
  ;[1 1 1] Input Binding
  (`SceneComponent.K2_AddLocalRotation` (`self.AzimuthGimbal`) (`KismetMathLibrary.MakeRotator` 0.0 0.0 AxisValue) false false))

(event `InputAxis|AimElevation`
  (params (AxisValue :type "Float (single-precision)"))
  ;[1 1 1] Input Binding
  (`SceneComponent.K2_AddLocalRotation` (`self.SpringArm`) (`KismetMathLibrary.MakeRotator` 0.0 AxisValue) false false))

(fn `UserConstructionScript`
  (`SceneComponent.K2_AttachToComponent` (`self.TankTurret`) (`self.TankBody`) "Turret" "SnapToTarget" "KeepRelative" "KeepRelative" true)
  (`SceneComponent.K2_AttachToComponent` (`self.TankBarrel`) (`self.TankTurret`) "Barrel" "KeepRelative" "KeepRelative" "KeepRelative" true)
  (`SceneComponent.K2_AttachToComponent` (`self.TankTrackLeft`) (`self.TankBody`) "TrackLeft" "KeepRelative" "KeepRelative" "KeepRelative" true)
  (`SceneComponent.K2_AttachToComponent` (`self.TankTrackRight`) (`self.TankBody`) "TrackRight" "KeepRelative" "KeepRelative" "KeepRelative" true))